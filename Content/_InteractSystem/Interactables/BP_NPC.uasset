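; BP_NPC is an interactable NPC actor for the interaction system, shown with a "To Talk" prompt.
; On Interact it snaps its pitch and yaw to face the interactor and plays a sound at its location, with no dialogue logic.
; Its getter functions supply the interaction type, message and InteractLocation position, with zero hold duration and tap count.
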(event EventBeginPlay)

(event Collision|EventActorBeginOverlap
  (params (OtherActor :type Actor%20Object%20Reference)))

(event EventTick
  (params (DeltaSeconds :type Float%20%28single-precision%29)))

(event EventInteract
  (params (Interactor :type Actor%20Object%20Reference))
  (bind _returnvalue (Transformation|GetActorLocation Interactor))
  (bind _returnvalue_2 (Transformation|GetActorLocation))
  (bind _returnvalue_3 (Math|Rotator|FindLookatRotation _returnvalue_2 _returnvalue))
  (Transformation|SetActorRotation (Math|Rotator|MakeRotator 0.0 (.pitch _returnvalue_3) (.yaw _returnvalue_3)))
  (Audio|PlaySoundatLocation "/Engine/VREditor/Sounds/UI/Object_Snaps_To_Grid.Object_Snaps_To_Grid" (Transformation|GetActorLocation) "0, 0, 0" 1.0 1.0 0.0 0 0 0 0))

(fn ConstructionScript)

(fn GetHoldDuration
  (return 0.0))

(fn GetInteractionType
  (return "NewEnumerator3"))

(fn GetInteractLocation
  (return (Transformation|GetWorldLocation (Variables|Default|GetInteractLocation))))

(fn GetInteractMessage
  (return "To Talk"))

(fn GetTapCount
  (return 0))