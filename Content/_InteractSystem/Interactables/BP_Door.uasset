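; Interactable door Blueprint that toggles between open and closed each time its Interact event fires.
; An IsOpen flag selects Open or Close, each of which updates the flag and plays its own sound at the door's location.
; A single timeline drives the DoorMesh's relative yaw, playing forward to open and reversing to close.
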(event Custom|Open
  (Variables|Default|SetIsOpen true)
  (Audio|PlaySoundatLocation "/Engine/VREditor/Sounds/UI/Enter_Simulate.Enter_Simulate" (Transformation|GetActorLocation) "0, 0, 0" 1.0 1.0 0.0 0 0 0 0)
  (bind _zrotation (Timeline|Open%20Timeline Play)
    (:Update
      (Transformation|SetRelativeRotation (Variables|Default|GetDoorMesh) (Math|Rotator|MakeRotator 0.0 0.0 _zrotation) false false))))

(event Custom|Close
  (Variables|Default|SetIsOpen false)
  (Audio|PlaySoundatLocation "/Engine/VREditor/Sounds/UI/Leave_Simulate.Leave_Simulate" (Transformation|GetActorLocation) "0, 0, 0" 1.0 1.0 0.0 0 0 0 0)
  (bind _zrotation (Timeline|Open%20Timeline Reverse)
    (:Update
      (Transformation|SetRelativeRotation (Variables|Default|GetDoorMesh) (Math|Rotator|MakeRotator 0.0 0.0 _zrotation) false false))))

(event EventInteract
  (params (Interactor :type Actor%20Object%20Reference))
  (if (Variables|Default|GetIsOpen)
    (CallFunction|Close)
    (else
      (CallFunction|Open))))

(fn ConstructionScript)