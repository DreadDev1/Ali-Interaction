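; BP_PickupItem is an interactable pickup in the interact system that an actor collects by interacting with it.
; On Interact it prints that the item was added to the interactor's inventory, plays a click sound at its location and destroys itself.
; The inventory addition is only a printed message, with no item actually stored.
; GetInteractionType returns its InteractionType variable.
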(event EventInteract
  (params (Interactor :type Actor%20Object%20Reference))
  (Development|PrintString (Utilities|String|ToString(Text) (Utilities|Text|FormatText "Added {Item Name}  to Inventory of {Actor Name}" (Utilities|GetDisplayName self) (Utilities|GetDisplayName Interactor))))
  (Audio|PlaySoundatLocation "/Engine/VREditor/Sounds/VR_click3.VR_click3" (Transformation|GetActorLocation) "0, 0, 0" 1.0 1.0 0.0 0 0 0 0)
  (Actor|DestroyActor))

(fn ConstructionScript)

(fn GetInteractionType
  (return (Variables|Default|GetInteractionType)))